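; BP_MixingBottle is an interactable bottle for potion mixing that changes color when the player uses a BP_ColorPotion on it.
; CheckColor searches the Recipes data table for the bottle and potion color pair in either order.
; A match sets the recipe's result color; otherwise LiquidGoPOOF sets a fixed fallback color.
; The ColorChanging timeline lerps the dynamic material between colors, with CanColor blocking mixing until it finishes.
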(event `self.ReceiveBeginPlay`
  (bind _staticmesh (`self.StaticMesh`))
  (`parent.ReceiveBeginPlay`)
  (bind _returnvalue (`PrimitiveComponent.CreateDynamicMaterialInstance` _staticmesh 0 (`PrimitiveComponent.GetMaterial` _staticmesh 0) "None"))
  (bind _output_get (set `self.MID_Bottle` _returnvalue))
  (`MaterialInstanceDynamic.SetVectorParameterValue` _output_get "Color" (`BlueprintMapLibrary.Map_Find` (`self.ColorsMaterial`) (`self.ColorInMixingBottle`))))

(event `Liquid Go POOF`
  (`KismetSystemLibrary.PrintString` "Color go POOF")
  (set `self.NewColorInMixingBottle` "NewEnumerator3")
  (set `self.CanColor?` false)
  (bind (_direction _alpha) (`Timeline|ColorChanging` :!via `PlayFromStart` :!label _label)
    (:`Update`
      (`self.ChangeColor` _alpha)
      (`KismetSystemLibrary.PrintString` (`|GetEnumeratorNameAsString` (`self.ColorInMixingBottle`))))
    (:`Finished`
      (set `self.CanColor?` true)
      (set `self.ColorInMixingBottle` (`self.NewColorInMixingBottle`))
      (`KismetSystemLibrary.PrintString` (`|GetEnumeratorNameAsString` (`self.ColorInMixingBottle`))))))

(event `PrintColor`
  (if (`self.FoundColorMatch`)
    (set `self.CanColor?` false)
    (goto _label :!via `PlayFromStart`)
    (else
      (`self.Liquid Go POOF`))))

(fn `ChangeColor`
  (params (Timeline :type "Float (double-precision)"))
  (`MaterialInstanceDynamic.SetVectorParameterValue` (`self.MID_Bottle`) "Color" (`KismetMathLibrary.LinearColorLerp` (`BlueprintMapLibrary.Map_Find` (`self.ColorsMaterial`) (`self.ColorInMixingBottle`)) (`self.GetNewLinearColor`) Timeline)))

(fn `CheckColor`
  (params (PotionInHand :type "/Game/BPs/PotionsMixing/test/BP_ColorPotion Object Reference"))
  (bind _colorinmixingbottle (`self.ColorInMixingBottle`))
  (bind _bottleinhandcolor (`self.BottleInHandColor`))
  (bind (_colorname _color1) (break `/Game/BPs/PotionsMixing/test/S_ColorRecipe` (`self.Out Row`)))
  (bind (_colorname_2 _color1_2 _color2) (break `/Game/BPs/PotionsMixing/test/S_ColorRecipe` (`self.Out Row`)))
  (bind _returnvalue (`|EnumEquality` _color1 _bottleinhandcolor))
  (set `self.BottleInHandColor` (`/Game/BPs/PotionsMixing/test/BP_ColorPotion.Color` PotionInHand))
  (bind _outrownames (`DataTableFunctionLibrary.GetDataTableRowNames` (`self.Recipes`)))
  (for _array_element _outrownames
    (bind _returnvalue_2 (`|GetDataTableRow` (`self.Recipes`) _array_element)
      (:`then`
        (set `self.Out Row` _returnvalue_2)
        (if (or (`|EnumEquality` _color1 _colorinmixingbottle) _returnvalue)
          (if (`|EnumEquality` (`.Color2_8_3815C9C44E5A611DCDADBB8ABE94CDB1` (break `/Game/BPs/PotionsMixing/test/S_ColorRecipe` (`self.Out Row`))) (select `bool` _returnvalue :`false` _bottleinhandcolor :`true` _colorinmixingbottle))
            (`KismetSystemLibrary.PrintString` (`|GetEnumeratorNameAsString` _color1_2))
            (`KismetSystemLibrary.PrintString` (`|GetEnumeratorNameAsString` _color2))
            (set `self.NewColorInMixingBottle` _colorname_2)
            (set `self.FoundColorMatch` true)
            (return)
            (else
              _)))
        (set `self.FoundColorMatch` false))))
  (return))

(fn `GetNewLinearColor`
  (returns (Value :type "LinearColor Structure"))
  (return (`BlueprintMapLibrary.Map_Find` (`self.ColorsMaterial`) (`self.NewColorInMixingBottle`))))

(fn `Interact`
  (params (`Player Character` :type "/Game/BPs/BP_FirstPersonCharacter Object Reference") (PickUpItem :type "/Game/BPs/BP_PickUpItem Object Reference"))
  (returns (UsedUpPickUp :type Boolean) (MultiUseItemused :type Boolean))
  (`/Engine/EditorBlueprintResources/StandardMacros.IsValid` PickUpItem
    (:`Is Valid`
      (bind _asbp_color_potion (cast `/Game/BPs/PotionsMixing/test/BP_ColorPotion` PickUpItem)
        (:`then`
          (if (`self.CanColor?`)
            (`self.CheckColor` _asbp_color_potion)
            (`self.PrintColor`)
            (return false true)))
        (:`CastFailed`
          (return false false))))))

(fn `UserConstructionScript`
  (`parent.UserConstructionScript`))