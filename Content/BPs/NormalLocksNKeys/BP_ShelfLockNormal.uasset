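; BP_ShelfLockNormal is a lock actor that opens when the player interacts with it while holding its matching key.
; Interact checks that the pick-up item is valid and equals the Key reference, then runs DestroyLock, destroys the key and reports it as used up.
; DestroyLock fires the Opened dispatcher, then destroys the lock after a short delay.
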(event `DestroyLock`
  (`self.Opened`)
  (`KismetSystemLibrary.Delay` 0.2)
  (`self.K2_DestroyActor`))

(fn `Interact`
  (params (`Player Character` :type "/Game/BPs/BP_FirstPersonCharacter Object Reference") (PickUpItem :type "/Game/BPs/BP_PickUpItem Object Reference"))
  (returns (UsedUpPickUp :type Boolean) (MultiUseItemused :type Boolean))
  (`/Engine/EditorBlueprintResources/StandardMacros.IsValid` PickUpItem
    (:`Is Valid`
      (if (== PickUpItem (`self.Key`))
        (`self.DestroyLock`)
        (`self.K2_DestroyActor` PickUpItem)
        (return true false)))))

(fn `UserConstructionScript`)