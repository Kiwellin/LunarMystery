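; BP_OfferingBowl is a sacrifice bowl that holds a single ingredient actor.
; AddIngredient, only when empty, disables the ingredient's capsule collision and snaps it to the ItemHere attach point.
; It also adds the ingredient to the show-only list of the player character's SceneCapture2D, using a character reference cached on BeginPlay.
; RemoveIngredient takes it off that list, destroys it and frees the bowl.
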(event `self.ReceiveBeginPlay`
  (`parent.ReceiveBeginPlay`)
  (bind _asbp_first_person_character (cast `/Game/BPs/BP_FirstPersonCharacter` (`GameplayStatics.GetPlayerCharacter` 0)))
  (set `self.Player Character` _asbp_first_person_character))

(event `AddIngredient`
  (params (Ingredient :type "/Game/BPs/Sacrifice/BP_Ingredient Object Reference"))
  (bind _addedingredient (`self.AddedIngredient`))
  (`/Engine/EditorBlueprintResources/StandardMacros.IsValid` _addedingredient
    (:`Is Not Valid`
      (bind _output_get (set `self.AddedIngredient` Ingredient))
      ; add ingredient to scene capture
      (`SceneCaptureComponent.ShowOnlyActorComponents` (`/Game/BPs/BP_FirstPersonCharacter.SceneCaptureComponent2D` (`self.Player Character`)) _output_get true)
      (`PrimitiveComponent.SetCollisionEnabled` (`/Game/BPs/Sacrifice/BP_Ingredient.Capsule` _addedingredient) "NoCollision")
      (`SceneComponent.K2_DetachFromComponent` (`Actor.RootComponent` Ingredient) "KeepRelative" "KeepRelative" "KeepRelative" true)
      (`self.K2_AttachToComponent` (`self.AddedIngredient`) (`self.ItemHere`) "None" "SnapToTarget" "SnapToTarget" "KeepWorld" true))))

(event `RemoveIngredient`
  (bind _addedingredient (`self.AddedIngredient`))
  (`/Engine/EditorBlueprintResources/StandardMacros.IsValid` _addedingredient
    (:`Is Valid`
      (`SceneCaptureComponent.RemoveShowOnlyActorComponents` (`/Game/BPs/BP_FirstPersonCharacter.SceneCaptureComponent2D` (`self.Player Character`)) _addedingredient true)
      (`PrimitiveComponent.SetCollisionEnabled` (`/Game/BPs/Sacrifice/BP_Ingredient.StaticMesh` _addedingredient) "QueryAndPhysics")
      (`SceneComponent.K2_DetachFromComponent` (`Actor.RootComponent` _addedingredient) "KeepRelative" "KeepRelative" "KeepRelative" true)
      (`self.K2_DestroyActor` (`self.AddedIngredient`))
      (set `self.AddedIngredient` null))))

(fn `UserConstructionScript`
  (`parent.UserConstructionScript`))