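; BP_Ingredient is an interactable herb ingredient that supplies copies of itself to an offering bowl.
; When Interact receives a valid BP_OfferingBowl as the pick-up item, it spawns a new actor of its own class.
; The copy's mesh comes from the HerbToSpawn map, keyed by class, and the copy goes to the bowl's AddIngredient.
; Neither the source ingredient nor the held bowl is consumed.
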(fn `Interact`
  (params (`Player Character` :type "/Game/BPs/BP_FirstPersonCharacter Object Reference") (PickUpItem :type "/Game/BPs/BP_PickUpItem Object Reference"))
  (returns (UsedUpPickUp :type Boolean) (MultiUseItemused :type Boolean))
  (bind _returnvalue (`GameplayStatics.GetObjectClass` self))
  (`/Engine/EditorBlueprintResources/StandardMacros.IsValid` PickUpItem
    (:`Is Valid`
      (bind _asbp_offering_bowl (cast `/Game/BPs/Sacrifice/BP_OfferingBowl` PickUpItem))
      (bind _returnvalue_2 (`|SpawnActorFromClass` _returnvalue (`self.Spawn Transform`) "AlwaysSpawn" "MultiplyWithRoot" null null))
      (`StaticMeshComponent.SetStaticMesh` (`/Game/BPs/Sacrifice/BP_Ingredient.StaticMesh` _returnvalue_2) (`BlueprintMapLibrary.Map_Find` (`self.HerbToSpawn`) _returnvalue))
      (`/Game/BPs/Sacrifice/BP_OfferingBowl.AddIngredient` _asbp_offering_bowl _returnvalue_2)
      (return false false))))

(fn `UserConstructionScript`)