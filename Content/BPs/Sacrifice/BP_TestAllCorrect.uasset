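; BP_TestAllCorrect is a sacrifice-puzzle controller that rewards the player with the last book key once enough correct offerings are made.
; On BeginPlay it hides the key and disables its collision.
; Each CheckIfAllCorrect call increments a counter; at five, it spawns a Niagara radial burst at its cylinder, reveals and moves the key to itself, then plays a level sequence after a short delay.
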(event `self.ReceiveBeginPlay`
  (bind _lastbookkey (`self.LastBookKey`))
  (`self.SetActorHiddenInGame` _lastbookkey true)
  (`self.SetActorEnableCollision` _lastbookkey false))

(event `CheckIfAllCorrect`
  (bind _lastbookkey (`self.LastBookKey`))
  (bind _output_get (set `self.CorrectOfferings` (+ (`self.CorrectOfferings`) 1)))
  (if (>= _output_get 5)
    (`NiagaraFunctionLibrary.SpawnSystemAtLocation` "/Niagara/DefaultAssets/Templates/Systems/RadialBurst.RadialBurst" (`SceneComponent.K2_GetComponentLocation` (`self.Cylinder`)) (struct) (0.5 0.5 0.5))
    (`self.SetActorHiddenInGame` _lastbookkey false)
    (`self.SetActorEnableCollision` _lastbookkey true)
    (`self.K2_SetActorLocation` _lastbookkey (`self.K2_GetActorLocation`) false false)
    (`KismetSystemLibrary.Delay` 0.1)
    (`MovieSceneSequencePlayer.Play` (`LevelSequenceActor.SequencePlayer` (`self.LS`)))))

(fn `UserConstructionScript`)