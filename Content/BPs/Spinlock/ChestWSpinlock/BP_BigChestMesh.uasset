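; BP_BigChestMesh is a chest that opens when its linked spinlock puzzle is solved.
; On BeginPlay it binds its OpenChest event to the Lock's solved-puzzle event, if the Lock reference is valid.
; OpenChest plays a timeline whose Lid and Latch tracks each drive a roll rotation on their own pivot components, swinging the lid and latch open.
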(event `self.ReceiveBeginPlay`
  (bind _lock (`self.Lock`))
  (`/Engine/EditorBlueprintResources/StandardMacros.IsValid` _lock
    (:`Is Valid`
      (add `/Game/BPs/Spinlock/BP_SpinLockPawn.SolvedPuzzle` _lock (delegate `OpenChest`)))))

(event `OpenChest`
  (bind (_direction _latch _lid) (`Timeline|Timeline`)
    (:`Update`
      (`SceneComponent.K2_SetRelativeRotation` (`self.PivotLid`) (`KismetMathLibrary.MakeRotator` (`KismetMathLibrary.Lerp` 0.0 -90.0 _lid)) false false)
      (`SceneComponent.K2_SetRelativeRotation` (`self.PivotLatch`) (`KismetMathLibrary.MakeRotator` (`KismetMathLibrary.Lerp` 0.0 -90.0 _latch)) false false))))

(fn `UserConstructionScript`)