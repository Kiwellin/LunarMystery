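; BP_BigChestLock is a spinlock puzzle for a big chest, extending a parent lock that the player possesses to operate.
; Interacting updates the selected piece's highlight, and a timeline fades a point light in on possession and back out on return to the character.
; Solving removes the input mapping, spawns an emitter and dissolves the lock through BPTransitionComponent, then runs the parent's solved logic and destroys the actor after the possess blend delay.
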(event `self.GetPossessed`
  (`parent.GetPossessed`)
  (bind (_direction _light) (`Timeline|TurnLightOn/Off` :!label _label)
    (:`Update`
      (`LightComponent.SetIntensity` (`self.PointLight`) (* _light (`self.LightMaxIntensity`))))))

(event `self.Return to Character`
  (`parent.Return to Character`)
  (goto _label :!via `Reverse`))

(event `self.ReceiveBeginPlay`
  (`parent.ReceiveBeginPlay`))

(event `self.SolvedSpinlock`
  (`self.RemoveMappingContext`)
  (`self.UpdateHighlightOfSelectedPiece` false)
  (`/Game/BPs/Niagara/BP_TransitionComponent.SpawnEmitter` (`self.BP_TransitionComponent`))
  (bind (_direction _newtrack_0) (`Timeline|DissolveLock`)
    (:`Update`
      (`/Game/BPs/Niagara/BP_TransitionComponent.DissolveObject` (`self.BP_TransitionComponent`) _newtrack_0))
    (:`Finished`
      (`parent.SolvedSpinlock`)
      (`KismetSystemLibrary.Delay` (`self.Smooth Possess Duration`))
      (`self.K2_DestroyActor`))))

(fn `Interact`
  (params (`Player Character` :type "/Game/BPs/BP_FirstPersonCharacter Object Reference") (PickUpItem :type "/Game/BPs/BP_PickUpItem Object Reference"))
  (returns (UsedUpPickUp :type Boolean) (MultiUseItemused :type Boolean))
  (bind _useduppickup (`parent.Interact` `Player Character` PickUpItem))
  (`self.UpdateHighlightOfSelectedPiece` (`self.CanBePossessed`))
  (return _useduppickup false))

(fn `UserConstructionScript`
  (`parent.UserConstructionScript`))