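; BP_well is an interactable well that starts spinning when given the correct item.
; Item interaction is deferred to the parent class, whose ItemIsCorrect event triggers Rotate here.
; Rotate plays the rope animation and runs a timeline that rolls PlaceBowlHere through three full turns.
; The timeline's Finished output loops back to replay both, so the motion repeats indefinitely.
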(event `self.ItemIsCorrect`
  (`parent.ItemIsCorrect`)
  (`self.Rotate`))

(event `Rotate`
  (set `self.StartLocationBucket` (`self.K2_GetActorRotation` (`self.Spinpart`)))
  (`SkeletalMeshComponent.Play` (`/Game/3D-Assets/Well/BP_WellRope.rope` (`self.rope`)) false :!label _label)
  (bind (_direction _newtrack_1) (`Timeline|Timeline` :!via `PlayFromStart`)
    (:`Update`
      (`SceneComponent.K2_SetRelativeRotation` (`self.PlaceBowlHere`) (`KismetMathLibrary.MakeRotator` (`KismetMathLibrary.Lerp` 0.0 1080.0 _newtrack_1)) false false))
    (:`Finished`
      (goto _label))))

(fn `Interact`
  (params (`Player Character` :type "/Game/BPs/BP_FirstPersonCharacter Object Reference") (PickUpItem :type "/Game/BPs/BP_PickUpItem Object Reference"))
  (returns (UsedUpPickUp :type Boolean) (MultiUseItemused :type Boolean))
  (bind (_useduppickup _multiuseitemused) (`parent.Interact` `Player Character` PickUpItem))
  (return _useduppickup _multiuseitemused))

(fn `UserConstructionScript`
  (`parent.UserConstructionScript`))