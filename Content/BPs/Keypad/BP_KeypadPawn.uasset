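; Keypad puzzle pawn that takes over from the player character on interact for entering a code.
; Navigation inputs step through a grid-ordered button array with wraparound, highlighting the selection via overlay material.
; Interact appends the selected label to the text display up to the code's length, or clears it on Cancel.
; Confirm returns to the character on a match, otherwise clears the display; exit input also returns.
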(event `self.ReceiveBeginPlay`
  ;[1 1 1] SETUP
  (set `self.Buttons` (`|MakeArray` (`self.Button_01`) (`self.Button_02`) (`self.Button_03`) (`self.Button_04`) (`self.Button_05`) (`self.Button_06`) (`self.Button_07`) (`self.Button_08`) (`self.Button_09`) (`self.Button_Cancel`) (`self.Button_00`) (`self.Button_Confirm`)))
  (`self.ClearDisplay`))

(event `/Game/BPs/interfaces/InteractionInterface.Interact`
  (params (`Player Character` :type "/Game/BPs/BP_FirstPersonCharacter Object Reference"))
  ;[1 1 1] Possess & Unpossess
  (`parent.Interact` `Player Character`)
  (`self.UpdateHighlightOfSelectedButton` true))

(event `EnhancedInput|/Game/Input/Actions/IA_ExitPuzzle`
  (params (ActionValue :type Boolean) (ElapsedSeconds :type "Float (double-precision)") (TriggeredSeconds :type "Float (double-precision)") (InputAction :type "InputAction Object Reference" :default "/Game/Input/Actions/IA_ExitPuzzle.IA_ExitPuzzle"))
  ;[1 1 1] Possess & Unpossess
  (:`Triggered`
    (`self.Return to Character`)))

(event `self.Return to Character`
  ;[1 1 1] Possess & Unpossess
  (`parent.Return to Character`)
  (`self.UpdateHighlightOfSelectedButton` false))

(event `EnhancedInput|/Game/Input/Actions/IA_NavigateRight`
  (params (ActionValue :type Boolean) (ElapsedSeconds :type "Float (double-precision)") (TriggeredSeconds :type "Float (double-precision)") (InputAction :type "InputAction Object Reference" :default "/Game/Input/Actions/IA_NavigateRight.IA_NavigateRight"))
  (:`Triggered`
    (`self.NavigateButtons` 1)))

(event `EnhancedInput|/Game/Input/Actions/IA_NavigateLeft`
  (params (ActionValue :type Boolean) (ElapsedSeconds :type "Float (double-precision)") (TriggeredSeconds :type "Float (double-precision)") (InputAction :type "InputAction Object Reference" :default "/Game/Input/Actions/IA_NavigateLeft.IA_NavigateLeft"))
  (:`Triggered`
    (`self.NavigateButtons` -1)))

(event `EnhancedInput|/Game/Input/Actions/IA_NavigateDown`
  (params (ActionValue :type Boolean) (ElapsedSeconds :type "Float (double-precision)") (TriggeredSeconds :type "Float (double-precision)") (InputAction :type "InputAction Object Reference" :default "/Game/Input/Actions/IA_NavigateDown.IA_NavigateDown"))
  (:`Triggered`
    (`self.NavigateButtons` 3)))

(event `EnhancedInput|/Game/Input/Actions/IA_NavigateUp`
  (params (ActionValue :type Boolean) (ElapsedSeconds :type "Float (double-precision)") (TriggeredSeconds :type "Float (double-precision)") (InputAction :type "InputAction Object Reference" :default "/Game/Input/Actions/IA_NavigateUp.IA_NavigateUp"))
  (:`Triggered`
    (`self.NavigateButtons` -3)))

(event `EnhancedInput|/Game/Input/Actions/IA_Interact`
  (params (ActionValue :type Boolean) (ElapsedSeconds :type "Float (double-precision)") (TriggeredSeconds :type "Float (double-precision)") (InputAction :type "InputAction Object Reference" :default "/Game/Input/Actions/IA_Interact.IA_Interact"))
  (:`Triggered`
    (if (== (`self.GetSelectedButton`) (`self.Button_Confirm`))
      ;[1 1 1] check if code true
      (if (`self.IsCodeCorrect`)
        (`self.Return to Character`)
        (else
          (`self.ClearDisplay`)))
      (else
        ;[1 1 1] Cancel button -> clear display
        (if (== (`self.GetSelectedButton`) (`self.Button_Cancel`))
          (`self.ClearDisplay`)
          (else
            ;[1 1 1] Add number to display
            (if (not (`self.IsCodeComplete`))
              (`self.AddToDisplay` (`/Game/BPs/Keypad/BP_KeypadButton.ButtonLabel` (`self.GetSelectedButton`))))))))))

(fn `AddToDisplay`
  (params (`b NumberToAdd` :type String))
  (bind _codedisplay (`self.CodeDisplay`))
  (`TextRenderComponent.K2_SetText` _codedisplay (`KismetTextLibrary.Conv_StringToText` (`KismetStringLibrary.Concat_StrStr` (`KismetTextLibrary.Conv_TextToString` (`TextRenderComponent.Text` _codedisplay)) `b NumberToAdd`))))

(fn `ClearDisplay`
  (`TextRenderComponent.K2_SetText` (`self.CodeDisplay`) (`KismetTextLibrary.Conv_StringToText` "")))

(fn `GetSelectedButton`
  (returns (Output :type "/Game/BPs/Keypad/BP_KeypadButton Object Reference"))
  (return (`|GetArrayItem` (`self.Buttons`) (`self.CurrentButtonIndex`))))

(fn `IsCodeComplete`
  (returns (ReturnValue :type Boolean))
  (return (== (`KismetStringLibrary.Len` (`KismetTextLibrary.Conv_TextToString` (`TextRenderComponent.Text` (`self.CodeDisplay`)))) (`KismetStringLibrary.Len` (`self.CorrectCode`)))))

(fn `IsCodeCorrect`
  (returns (ReturnValue :type Boolean))
  (return (`KismetStringLibrary.EqualEqual_StrStr` (`KismetTextLibrary.Conv_TextToString` (`TextRenderComponent.Text` (`self.CodeDisplay`))) (`self.CorrectCode`))))

(fn `NavigateButtons`
  (params (Direction :type Integer))
  (`self.UpdateHighlightOfSelectedButton` false)
  (set `self.CurrentButtonIndex` (+ (`self.CurrentButtonIndex`) Direction))
  (`|ExecutionSequence`
    (:`then_0`
      ;[1 1 1] Make sure index not too high
      (if (> (`self.CurrentButtonIndex`) (`KismetArrayLibrary.Array_LastIndex` (`self.Buttons`)))
        (set `self.CurrentButtonIndex` (- (`self.CurrentButtonIndex`) (`KismetArrayLibrary.Array_Length` (`self.Buttons`))))))
    (:`then_1`
      ;[1 1 1] Make sure index not too low
      (if (< (`self.CurrentButtonIndex`) 0)
        (set `self.CurrentButtonIndex` (+ (`self.CurrentButtonIndex`) (`KismetArrayLibrary.Array_Length` (`self.Buttons`))))))
    (:`then_2`
      ;[1 1 1] Update highlight
      (`self.UpdateHighlightOfSelectedButton` true))))

(fn `UpdateHighlightOfSelectedButton`
  (params (bEnabled :type Boolean))
  (`MeshComponent.SetOverlayMaterial` (`self.GetSelectedButton`) (select `bool` bEnabled :`true` "/Game/Materials/MI_ButtonHighlight.MI_ButtonHighlight" :!type "MaterialInterface Object Reference")))

(fn `UserConstructionScript`)