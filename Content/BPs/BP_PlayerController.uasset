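; Player controller that switches Enhanced Input mapping contexts as the game moves through its tutorial.
; BeginPlay adds the first tutorial mapping, then ChangeMapping adds either the second tutorial mapping or, once tutorials are done, the first-person mapping.
; Contexts are all added at priority 0 without removing earlier ones.
; The Possess event is empty, and the logic caching the first-person character is disconnected.
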(event `self.ReceivePossess`
  (params (PossessedPawn :type "Pawn Object Reference")))

(event `self.ReceiveBeginPlay`
  (`EnhancedInputSubsystemInterface.AddMappingContext` (subsystem `EnhancedInputLocalPlayerSubsystem`) (`self.TutorialMapping 1`) 0 (struct)))

(event `ChangeMapping`
  (params (`TutorialsDone?` :type Boolean))
  (`EnhancedInputSubsystemInterface.AddMappingContext` (subsystem `EnhancedInputLocalPlayerSubsystem`) (select `bool` `TutorialsDone?` :`false` (`self.TutorialMapping 2`) :`true` (`self.FirstPersonMapping`)) 0 (struct)))

(fn `UserConstructionScript`)