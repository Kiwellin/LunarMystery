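; BP_AnimalMathBox is a prototype puzzle box that opens when its spinlock is solved.
; The first interaction detaches it, teleports it to a preset location and makes the Spinlock possessable; later interactions pass to the Spinlock.
; Solving fires DestroyActor, which, despite its name, animates lid and latch by timeline, then disables collision on box and attached actors, except BP_Bookkey, which it detaches.
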(event `self.ReceiveBeginPlay`
  (add `/Game/BPs/Spinlock/BP_SpinLockPawn.SolvedPuzzle` (`self.Spinlock`) (delegate `DestroyActor`)))

(event `DestroyActor`
  (bind (_direction _latch _lid) (`Timeline|Timeline`)
    (:`Update`
      (`SceneComponent.K2_SetRelativeRotation` (`self.Scene`) (`KismetMathLibrary.MakeRotator` (`KismetMathLibrary.Lerp` 0.0 -90.0 _lid)) false false)
      (`SceneComponent.K2_SetRelativeRotation` (`self.Scene1`) (`KismetMathLibrary.MakeRotator` (`KismetMathLibrary.Lerp` 0.0 -90.0 _latch)) false false))
    (:`Finished`
      (for _array_element (`self.GetAttachedActors` self true false)
        (bind _asbp_bookkey (cast `/Game/BPs/BookBox/BP_Bookkey` _array_element)
          (:`then`
            (`self.K2_DetachFromActor` _asbp_bookkey "KeepWorld" "KeepWorld" "KeepWorld"))
          (:`CastFailed`
            (`self.SetActorEnableCollision` _array_element false))))
      (`self.SetActorEnableCollision` false))))

(event `MoveBoxOnDrawer`
  (`self.K2_SetActorLocation` (`SceneComponent.K2_GetComponentLocation` (`self.NewLocation`))))

(fn `Interact`
  (params (`Player Character` :type "/Game/BPs/BP_FirstPersonCharacter Object Reference") (PickUpItem :type "/Game/BPs/BP_PickUpItem Object Reference"))
  (returns (UsedUpPickUp :type Boolean) (MultiUseItemused :type Boolean))
  (bind _spinlock (`self.Spinlock`))
  (if (`self.Moved?`)
    (`/Game/BPs/interfaces/InteractionInterface.Interact` _spinlock `Player Character` PickUpItem)
    (else
      (set `/Game/BPs/BP_InteractablePossessable.CanBePossessed` true _spinlock)
      (`self.K2_DetachFromActor` "KeepWorld" "KeepWorld" "KeepWorld")
      (`self.MoveBoxOnDrawer`)
      (set `self.Moved?` true)
      (return false false))))

(fn `UserConstructionScript`)