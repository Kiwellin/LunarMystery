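; BP_Dirt is an interactable dirt pile that is cleared when the player uses the correct item on it.
; Interact compares the held pickup to CorrectItem; a match destroys both the item and, after a short delay, the dirt, and reports the pickup as used up.
; A missing or wrong item sends a hint or a random wrong-item line to the player's HUD dialogue.
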(event `DESTROY`
  (`KismetSystemLibrary.Delay` 0.1)
  (`self.K2_DestroyActor`))

(event `/Game/BPs/interfaces/BPI_ItemDialogueTextInterface.UpdateDisplayText`
  (params (PlayerCharacter :type "/Game/BPs/BP_FirstPersonCharacter Object Reference") (TypeOfText :type "/Game/BPs/interfaces/E_DialogueTypes Enum" :default "NewEnumerator0"))
  (bind _ingamehud (`/Game/BPs/BP_FirstPersonCharacter.IngameHUD` PlayerCharacter))
  (switch `/Game/BPs/interfaces/E_DialogueTypes` TypeOfText
    (:`NewEnumerator0`
      (set `self.Text` "It looks like there is something beneath the dirt"))
    (:`NewEnumerator1`
      (set `self.Text` (`KismetArrayLibrary.Array_Random` (`self.WrongItemDialogue`))))
    (:`NewEnumerator2`
      (set `self.Text` "")))
  (`/Game/BPs/Widgets/ComicsAndTuts/BP_Controlls.SetFulltext` _ingamehud (`self.Text`))
  (`/Game/BPs/Widgets/ComicsAndTuts/BP_Controlls.UpdateDialogueText` _ingamehud))

(fn `Interact`
  (params (`Player Character` :type "/Game/BPs/BP_FirstPersonCharacter Object Reference") (PickUpItem :type "/Game/BPs/BP_PickUpItem Object Reference"))
  (returns (UsedUpPickUp :type Boolean) (MultiUseItemused :type Boolean))
  (`/Engine/EditorBlueprintResources/StandardMacros.IsValid` PickUpItem
    (:`Is Valid`
      (if (== PickUpItem (`self.CorrectItem`))
        (`self.K2_DestroyActor` PickUpItem)
        (`self.DESTROY`)
        (return true false)
        (else
          (`self.UpdateDisplayText` `Player Character` "NewEnumerator1"))))
    (:`Is Not Valid`
      (`self.UpdateDisplayText` `Player Character`)))
  (return false false))

(fn `UserConstructionScript`)