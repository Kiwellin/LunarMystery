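; Tutorial trigger actor that detects when the player looks toward it and completes the look tutorial step.
; On BeginPlay it caches the first-person character and starts a looping timer instead of using Tick or overlap.
; Each check compares camera forward with the direction to the actor by dot product, ignoring distance and occlusion.
; Above a threshold it calls LookTutDone on the character, then destroys itself after a short delay.
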(event `self.ReceiveBeginPlay`
  (bind _asbp_first_person_character (cast `/Game/BPs/BP_FirstPersonCharacter` (`GameplayStatics.GetPlayerCharacter` 0)))
  (set `self.As BP First Person Character` _asbp_first_person_character)
  (`KismetSystemLibrary.K2_SetTimerDelegate` (delegate `CheckIfPlayerLooking at`) 0.1 true))

(event `CheckIfPlayerLooking at`
  (bind _as_bp_first_person_character (`self.As BP First Person Character`))
  (if (>= (* (`KismetMathLibrary.Dot_VectorVector` (`KismetMathLibrary.GetForwardVector` (`KismetMathLibrary.FindLookAtRotation` (`self.K2_GetActorLocation` self) (`self.K2_GetActorLocation` _as_bp_first_person_character))) (`SceneComponent.GetForwardVector` (`/Game/BPs/BP_FirstPersonCharacter.Camera` _as_bp_first_person_character))) -1.0) 0.9)
    (`/Game/BPs/BP_FirstPersonCharacter.LookTutDone` (`self.As BP First Person Character`))
    (`KismetSystemLibrary.Delay` 0.2)
    (`self.K2_DestroyActor`)))

(fn `UserConstructionScript`)