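; BP_Pin is a placement target for items, including hint notes, that reacts when the correct item is placed.
; ItemIsCorrect fires the all-correct check and placed-correct calls, then disables the item's collision if it cannot be picked up again.
; For re-pickable items on a note hint pin, it shifts the BP_HintNote mesh vertically by its PinLoc's relative Y.
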(event `self.ItemIsCorrect`
  (`self.CheckIfAllCorrect`)
  (`self.ItemPlacedCorrect`)
  (if (`self.CanPickUpItemAgain`)
    (if (`self.TargetIsNote/HintPin?`)
      (bind _asbp_hint_note (cast `/Game/BPs/HintsAndNotes/BP_HintNote` (`self.PlacedItem`)))
      (bind (_relativelocation_x _relativelocation_y) (`KismetMathLibrary.BreakVector` (`SceneComponent.RelativeLocation` (`/Game/BPs/HintsAndNotes/BP_HintNote.PinLoc` _asbp_hint_note))))
      (`SceneComponent.K2_AddWorldOffset` (`/Game/BPs/BP_PickUpItem.StaticMesh` _asbp_hint_note) (`KismetMathLibrary.MakeVector` 0.0 0.0 _relativelocation_y) false false))
    (else
      (`self.SetActorEnableCollision` (`self.PlacedItem`) false))))

(fn `UserConstructionScript`
  (`parent.UserConstructionScript`))