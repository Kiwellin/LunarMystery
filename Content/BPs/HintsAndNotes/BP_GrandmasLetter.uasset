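; BP_GrandmasLetter is a letter actor in the hints and notes set that ends the tutorial when first interacted with.
; It overrides ChangeParents, calling the parent behavior and then, guarded by FirstInteractDone and a DoOnce, calling TutEnd on the BP_FirstPersonCharacter player.
; The event graph and construction script add no logic of their own.
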(fn `ChangeParents`
  (params (Parent :type "SceneComponent Object Reference"))
  (`parent.ChangeParents` Parent)
  (if (not (`self.First interact Done?`))
    (`/Engine/EditorBlueprintResources/StandardMacros.DoOnce` false
      (:`Completed`
        (set `self.First interact Done?` true)
        (bind _asbp_first_person_character (cast `/Game/BPs/BP_FirstPersonCharacter` (`GameplayStatics.GetPlayerCharacter` 0)))
        (`/Game/BPs/BP_FirstPersonCharacter.Tut End` _asbp_first_person_character)))))

(fn `UserConstructionScript`
  (`parent.UserConstructionScript`))