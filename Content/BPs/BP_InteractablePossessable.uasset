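; Base interactable that the player character can possess and later leave, expecting child classes to supply a camera.
; Interact triggers possession if allowed, hiding the HUD, swapping Enhanced Input mapping contexts and blending the view before possessing.
; Returning reverses this after repositioning the character.
; Placement takes yaw from the camera and traces down from it, or from an optional BP_UnpossessPuzzlePosition component, to set the capsule on the surface.
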(event `GetPossessed`
  (bind _player_character (`self.Player Character`))
  ;[0.5599 0.5599 0.5599] Get Possessed
  (`/Game/BPs/BP_FirstPersonCharacter.StopCamShake` _player_character)
  (`Widget.SetVisibility` (`/Game/BPs/BP_FirstPersonCharacter.IngameHUD` _player_character) "Collapsed")
  (`EnhancedInputSubsystemInterface.RemoveMappingContext` (pcsubsystem `EnhancedInputLocalPlayerSubsystem` (`GameplayStatics.GetPlayerController` 0)) (`self.CharacterMappingContext`) (struct))
  (`PlayerController.SetViewTargetWithBlend` (`GameplayStatics.GetPlayerController` 0) self (`self.Smooth Possess Duration`) (`self.Blend Func`) (`self.Blend Exp`) false)
  (`KismetSystemLibrary.Delay` (`self.Smooth Possess Duration`))
  (`Controller.Possess` (`GameplayStatics.GetPlayerController` 0) self)
  (`EnhancedInputSubsystemInterface.AddMappingContext` (pcsubsystem `EnhancedInputLocalPlayerSubsystem` (`GameplayStatics.GetPlayerController` 0)) (`self.Mapping Context`) 0 (struct)))

(event `Return to Character`
  (bind _player_character (`self.Player Character`))
  ;[1 1 1] Get Unpossessed
  (`self.PositionPlayerCharacter`)
  (`EnhancedInputSubsystemInterface.RemoveMappingContext` (pcsubsystem `EnhancedInputLocalPlayerSubsystem` (`GameplayStatics.GetPlayerController` 0)) (`self.Mapping Context`) (struct))
  (`PlayerController.SetViewTargetWithBlend` (`GameplayStatics.GetPlayerController` 0) (`self.Player Character`) (`self.Smooth Possess Duration`) (`self.Blend Func`) (`self.Blend Exp`) false)
  (`KismetSystemLibrary.Delay` (`self.Smooth Possess Duration`))
  (`EnhancedInputSubsystemInterface.AddMappingContext` (pcsubsystem `EnhancedInputLocalPlayerSubsystem` (`GameplayStatics.GetPlayerController` 0)) (`self.CharacterMappingContext`) 0 (struct))
  (`Controller.Possess` (`GameplayStatics.GetPlayerController` 0) _player_character)
  (`Widget.SetVisibility` (`/Game/BPs/BP_FirstPersonCharacter.IngameHUD` _player_character) "Visible"))

(fn `Interact`
  (params (`Player Character` :type "/Game/BPs/BP_FirstPersonCharacter Object Reference") (PickUpItem :type "/Game/BPs/BP_PickUpItem Object Reference"))
  (returns (UsedUpPickUp :type Boolean) (MultiUseItemused :type Boolean))
  (set `self.Player Character` `Player Character`)
  (if (`self.CanBePossessed`)
    (`self.GetPossessed`)
    (return false false)))

(fn `PositionPlayerCharacter`
  (locals (Camera :type "CameraComponent Object Reference") (LineTraceStart :type "Vector Structure" :default (0.0 0.0 0.0)) (LineTraceEnd :type "Vector Structure" :default (0.0 0.0 0.0)))
  (bind _returnvalue (`self.GetComponentByClass` self "/Game/BPs/Components/BP_UnpossessPuzzlePosition.BP_UnpossessPuzzlePosition_C"))
  (bind (_returnvalue_roll _returnvalue_pitch _returnvalue_yaw) (`KismetMathLibrary.BreakRotator` (`SceneComponent.K2_GetComponentRotation` (`local.Camera`))))
  (bind (_returnvalue_roll_2 _returnvalue_pitch_2 _returnvalue_yaw_2) (`KismetMathLibrary.BreakRotator` (`SceneComponent.K2_GetComponentRotation` (`local.Camera`))))
  (bind _returnvalue_2 (`SceneComponent.K2_GetComponentLocation` (`local.Camera`)))
  (bind _output_get (set `local.Camera` (`self.GetComponentByClass` "/Script/Engine.CameraComponent")))
  (`/Engine/EditorBlueprintResources/StandardMacros.IsValid` _output_get
    (:`Is Valid`
      (`/Engine/EditorBlueprintResources/StandardMacros.IsValid` _returnvalue
        (:`Is Valid`
          (`self.K2_SetActorRotation` (`self.Player Character`) (`KismetMathLibrary.MakeRotator` _returnvalue_roll 0.0 _returnvalue_yaw) false)
          (set `local.LineTraceStart` (`SceneComponent.K2_GetComponentLocation` _returnvalue))
          (set `local.LineTraceEnd` (- (`SceneComponent.K2_GetComponentLocation` (`self.GetComponentByClass` "/Game/BPs/Components/BP_UnpossessPuzzlePosition.BP_UnpossessPuzzlePosition_C")) (0.0 0.0 300.0))))
        (:`Is Not Valid`
          (`self.K2_SetActorRotation` (`self.Player Character`) (`KismetMathLibrary.MakeRotator` 0.0 0.0 _returnvalue_yaw_2) false)
          (set `local.LineTraceStart` _returnvalue_2)
          (set `local.LineTraceEnd` (- _returnvalue_2 (0.0 0.0 600.0)))))
      (bind (_outhit _returnvalue_3) (`KismetSystemLibrary.LineTraceSingleForObjects` :`Start` (`local.LineTraceStart`) :`End` (`local.LineTraceEnd`) :`ObjectTypes` (`|MakeArray` "ObjectTypeQuery1" "ObjectTypeQuery2" :!type "EObjectTypeQuery Enum") :`DrawDebugType` "ForDuration" :`DrawTime` 10.0))
      (if _returnvalue_3
        (`self.K2_SetActorLocation` (`self.Player Character`) (+ (`.Location` (`GameplayStatics.BreakHitResult` _outhit)) (`KismetMathLibrary.MakeVector` 0.0 0.0 (+ (`CapsuleComponent.CapsuleHalfHeight` (`Character.CapsuleComponent` (`self.Player Character`))) 1.0))) false false)))
    (:`Is Not Valid`
      (`KismetSystemLibrary.PrintString` "BP_InteractablePossessablee assumes childe has camera component but found none!" true true (struct :`R` 0.705729 :`G` 0.01713 :`A` 1.0) 5.0))))

(fn `UserConstructionScript`)