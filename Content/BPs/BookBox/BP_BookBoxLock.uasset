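; BP_BookBoxLock is a book box lock that accepts a key item of the correct class through Interact and uses it up.
; If the item cannot be picked up again, ItemIsCorrect disables its collision and a timeline turns its mesh a quarter turn.
; Transition components on the lock and BP_Bookkey then spawn emitters and dissolve both, after which the lock calls CallUnlocked and destroys itself.
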(event `self.ItemIsCorrect`
  (if (not (`self.CanPickUpItemAgain`))
    (`self.SetActorEnableCollision` (`self.PlacedItem`) false)
    (bind (_direction _newtrack_0) (`Timeline|Timeline` :!via `PlayFromStart`)
      (:`Update`
        (`SceneComponent.K2_SetRelativeRotation` (`/Game/BPs/BP_PickUpItem.StaticMesh` (`self.PlacedItem`)) (`KismetMathLibrary.MakeRotator` 0.0 0.0 (`KismetMathLibrary.Lerp` 0.0 90.0 _newtrack_0)) false false))
      (:`Finished`
        (bind _asbp_bookkey (cast `/Game/BPs/BookBox/BP_Bookkey` (`self.PlacedItem`)))
        (`/Game/BPs/Niagara/BP_TransitionComponent.SpawnEmitter` (`self.BP_TransitionComponent`))
        (`/Game/BPs/Niagara/BP_TransitionComponent.SpawnEmitter` (`/Game/BPs/BookBox/BP_Bookkey.BP_TransitionComponent` _asbp_bookkey))
        (bind (_direction_2 _newtrack_0_2) (`Timeline|Timeline_0`)
          (:`Update`
            (`/Game/BPs/Niagara/BP_TransitionComponent.DissolveObject` (`self.BP_TransitionComponent`) _newtrack_0_2)
            (`/Game/BPs/Niagara/BP_TransitionComponent.DissolveObject` (`/Game/BPs/BookBox/BP_Bookkey.BP_TransitionComponent` _asbp_bookkey) _newtrack_0_2))
          (:`Finished`
            (`self.Unlocked`)
            (`self.K2_DestroyActor`)))))))

(fn `Interact`
  (params (`Player Character` :type "/Game/BPs/BP_FirstPersonCharacter Object Reference") (PickUpItem :type "/Game/BPs/BP_PickUpItem Object Reference"))
  (returns (UsedUpPickUp :type Boolean) (MultiUseItemused :type Boolean))
  (`/Engine/EditorBlueprintResources/StandardMacros.IsValid` PickUpItem
    (:`Is Valid`
      (if (`self.ItemCorrect`)
        _
        (elif (== (`GameplayStatics.GetObjectClass` PickUpItem) (`self.CorrecItemClass`))
          (`KismetSystemLibrary.PrintString` "calss correct")
          (`self.PlaceItem` PickUpItem)
          (`self.ItemIsCorrect`)
          (set `self.ItemCorrect` true)
          (return true false)
          (else
            (`KismetSystemLibrary.PrintString` "class not correct")))))
    (:`Is Not Valid`
      (`KismetSystemLibrary.PrintString` "no pick up found"))))

(fn `UserConstructionScript`
  (`parent.UserConstructionScript`))