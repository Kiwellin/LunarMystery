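; BP_BookBox is an actor, apparently a locked book box, that dissolves away once its three locks are opened.
; On BeginPlay it binds to the unlock event of each lock and counts unlocks as they arrive.
; At three, BPTransitionComponent spawns an emitter and a timeline drives its dissolve effect, then the actor destroys itself after a short delay.
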(event `self.ReceiveBeginPlay`
  (add `/Game/BPs/BookBox/BP_BookBoxLock.Unlocked` (`self.Lock_01`) (delegate `AddCorrect`))
  (add `/Game/BPs/BookBox/BP_BookBoxLock.Unlocked` (`self.Lock_02`) (delegate `AddCorrect`))
  (add `/Game/BPs/BookBox/BP_BookBoxLock.Unlocked` (`self.Lock_03`) (delegate `AddCorrect`)))

(event `AddCorrect`
  (set `self.LocksUnlocked` (+ (`self.LocksUnlocked`) 1))
  (`self.CheckLockAmount`))

(event `CheckLockAmount`
  (if (== (`self.LocksUnlocked`) 3)
    (`/Game/BPs/Niagara/BP_TransitionComponent.SpawnEmitter` (`self.BP_TransitionComponent`))
    (bind (_direction _newtrack_0) (`Timeline|Timeline`)
      (:`Update`
        (`/Game/BPs/Niagara/BP_TransitionComponent.DissolveObject` (`self.BP_TransitionComponent`) _newtrack_0))
      (:`Finished`
        (`KismetSystemLibrary.Delay` 0.2)
        (`self.K2_DestroyActor`)))))

(fn `UserConstructionScript`)