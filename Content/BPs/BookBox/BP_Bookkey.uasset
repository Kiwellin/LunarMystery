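; BP_Bookkey is a key actor in the BookBox set that starts out attached to a bucket.
; On BeginPlay it runs parent logic, then, if its Bucket reference is valid, attaches to that bucket's Bucket component at Socket0.
; The attachment snaps location to the socket while keeping world rotation and relative scale; any other behavior comes from the parent class.
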(event `self.ReceiveBeginPlay`
  (bind _bucket (`self.Bucket`))
  (`parent.ReceiveBeginPlay`)
  (`/Engine/EditorBlueprintResources/StandardMacros.IsValid` _bucket
    (:`Is Valid`
      (`self.K2_AttachToComponent` (`/Game/3D-Assets/Well/BP_WellRope.Bucket` _bucket) "Socket0" "SnapToTarget" "KeepWorld" "KeepRelative"))))

(fn `UserConstructionScript`
  (`parent.UserConstructionScript`))