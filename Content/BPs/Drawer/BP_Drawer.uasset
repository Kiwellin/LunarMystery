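; BP_Drawer is an interactable drawer that slides open and shut along its forward vector.
; BeginPlay caches the closed position and computes the open one from OpenLength.
; Interact toggles Open, then calls the TIMELINE event, which plays or reverses a timeline that lerps actor location between the two.
; CanOpen acts as a busy lock during movement, though Open still toggles on every interaction.
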(event `self.ReceiveBeginPlay`
  (bind (_returnvalue_location _returnvalue_rotation) (`KismetMathLibrary.BreakTransform` (`self.GetTransform`)))
  (bind _output_get (set `self.StartLocation` _returnvalue_location))
  (set `self.EndLocation` (+ _output_get (* (`KismetMathLibrary.GetForwardVector` _returnvalue_rotation) (`self.OpenLength`)))))

(event `TIMELINE`
  (if (not (`self.Can open?`))
    (set `self.Can open?` true)
    (if (`self.Open?`)
      (set `self.Open?` true)
      (bind (_direction _newtrack_0) (`Timeline|Timeline_0` :!label _label)
        (:`Update`
          (`self.K2_SetActorLocation` (`KismetMathLibrary.VLerp` (`self.StartLocation`) (`self.EndLocation`) _newtrack_0)))
        (:`Finished`
          (set `self.Can open?` false)))
      (else
        (set `self.Open?` false)
        (goto _label :!via `Reverse`)))))

(fn `Interact`
  (params (`Player Character` :type "/Game/BPs/BP_FirstPersonCharacter Object Reference") (PickUpItem :type "/Game/BPs/BP_PickUpItem Object Reference"))
  (returns (UsedUpPickUp :type Boolean) (MultiUseItemused :type Boolean))
  (if (`self.Open?`)
    (set `self.Open?` false)
    (else
      (set `self.Open?` true)))
  (`self.TIMELINE`)
  (return false false))

(fn `UserConstructionScript`)