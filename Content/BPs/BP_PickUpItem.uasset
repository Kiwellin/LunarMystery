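; BP_PickUpItem is an item actor that can be attached to a parent component, dropped back into the world, or destroyed.
; ChangeParents turns off the mesh's physics, CCD and collision, then detaches and snaps it to the given parent, keeping world scale.
; Drop detaches in place and restores collision, physics simulation and CCD.
; Actor tick is enabled only while attached, though the Blueprint has no active Tick logic.
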(event `self.ReceiveBeginPlay`
  (`self.SetActorTickEnabled` false))

(event `Drop`
  (bind _staticmesh (`self.StaticMesh`))
  (`self.K2_DetachFromActor` "KeepWorld" "KeepWorld" "KeepWorld")
  (`PrimitiveComponent.SetCollisionEnabled` (`self.StaticMesh`) "QueryAndPhysics")
  (`PrimitiveComponent.SetSimulatePhysics` _staticmesh true)
  (`PrimitiveComponent.SetUseCCD` _staticmesh true "None")
  (`self.SetActorTickEnabled` false))

(fn `ChangeParents`
  (params (Parent :type "SceneComponent Object Reference"))
  (bind _staticmesh (`self.StaticMesh`))
  (`PrimitiveComponent.SetSimulatePhysics` _staticmesh false)
  (`PrimitiveComponent.SetUseCCD` _staticmesh false "None")
  (`PrimitiveComponent.SetCollisionEnabled` (`self.StaticMesh`) "NoCollision")
  (`SceneComponent.K2_DetachFromComponent` (`self.RootComponent`) "KeepRelative" "KeepRelative" "KeepWorld" true)
  (`self.K2_AttachToComponent` Parent "None" "SnapToTarget" "SnapToTarget" "KeepWorld")
  (`self.SetActorTickEnabled` true))

(fn `DestroySelf`
  (`self.K2_DestroyActor`))

(fn `UserConstructionScript`)