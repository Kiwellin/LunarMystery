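; Statue rotation puzzle that opens a secret compartment once three linked statues all face correctly.
; Each statue's GiveRotationBool dispatcher updates its slot in RotArray, and CheckRotations fires the puzzle-solved event when every entry is true.
; Solving plays a Level Sequence and disables statue interaction; a separate SpawnItem/OpenLatch event unhides the hidden object and enables its collision.
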(event `self.ReceiveBeginPlay`
  (`parent.ReceiveBeginPlay`)
  (add `self.GiveRotationBool` (`self.Statue_1`) (delegate `GiveRotationBool_Event`))
  (add `self.GiveRotationBool` (`self.Statue_2`) (delegate `GiveRotationBool_Event_0`))
  (add `self.GiveRotationBool` (`self.Statue_3`) (delegate `GiveRotationBool_Event_1`))
  (set `self.RotArray` (`|MakeArray` (`self.StatueRot_1`) (`self.StatueRot_2`) (`self.StatueRot_3`))))

(event `GiveRotationBool_Event` :!signature `self.GiveRotationBool`
  (params (`IsRotCorrect?` :type Boolean))
  (bind _output_get (set `self.StatueRot_1` `IsRotCorrect?`))
  (`KismetArrayLibrary.Array_Set` (`self.RotArray`) 0 _output_get)
  (`self.CheckIfAllCorrect` false :!label _label))

(event `GiveRotationBool_Event_0` :!signature `self.GiveRotationBool`
  (params (`IsRotCorrect?` :type Boolean))
  (bind _output_get (set `self.StatueRot_2` `IsRotCorrect?`))
  (`KismetArrayLibrary.Array_Set` (`self.RotArray`) 1 _output_get)
  (goto _label))

(event `GiveRotationBool_Event_1` :!signature `self.GiveRotationBool`
  (params (`IsRotCorrect?` :type Boolean))
  (bind _output_get (set `self.StatueRot_3` `IsRotCorrect?`))
  (`KismetArrayLibrary.Array_Set` (`self.RotArray`) 2 _output_get)
  (goto _label))

(event `CheckIfAllCorrect`
  (params (NewParam :type Boolean) (CorrectStatue :type "/Game/BPs/Statues/BP_StatuesRotate Object Reference"))
  (bind _all_correct (`self.CheckRotations`))
  (if _all_correct
    (`KismetSystemLibrary.PrintString` "all 3 correct")
    (`self.PuzzleSolved_Event`)))

(event `PuzzleSolved_Event`
  (`MovieSceneSequencePlayer.Play` (`LevelSequenceActor.SequencePlayer` (`self.LevelSequence`)))
  (set `/Game/BPs/Statues/BP_StatuesRotate.CanBeInteractedW` false (`self.Statue_1`))
  (set `/Game/BPs/Statues/BP_StatuesRotate.CanBeInteractedW` false (`self.Statue_2`))
  (set `/Game/BPs/Statues/BP_StatuesRotate.CanBeInteractedW` false (`self.Statue_3`)))

(event `SpawnItem/OpenLatch`
  (bind _object_to_unhide (`self.Object To Unhide`))
  (`self.SetActorHiddenInGame` _object_to_unhide false)
  (`self.SetActorEnableCollision` _object_to_unhide true))

(fn `CheckRotations`
  (returns (`All Correct` :type Boolean))
  (for _array_element (`self.RotArray`)
    (if (== _array_element false)
      (`KismetSystemLibrary.PrintString` (`KismetStringLibrary.Conv_BoolToString` _array_element))
      (return false)))
  (return true))

(fn `Interact`
  (params (`Player Character` :type "/Game/BPs/BP_FirstPersonCharacter Object Reference") (PickUpItem :type "/Game/BPs/BP_PickUpItem Object Reference"))
  (returns (UsedUpPickUp :type Boolean) (MultiUseItemused :type Boolean))
  (bind _useduppickup (`parent.Interact` `Player Character` PickUpItem))
  (return _useduppickup false))

(fn `UserConstructionScript`
  (`parent.UserConstructionScript`))