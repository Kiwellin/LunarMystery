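; Rotatable puzzle statue that can require a specific item before interacting spins it in 45-degree steps.
; Spin direction comes from a dot product between the camera's right vector and direction to the statue; Tick lerps the cylinder toward the target yaw.
; After each spin it compares against the correct rotation, plays sounds and broadcasts the result.
; It also shows wrong-item HUD dialogue and has a timeline-driven lid opening.
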(event `self.ReceiveBeginPlay`
  (bind (_relativerotation_roll _relativerotation_pitch _relativerotation_yaw) (`KismetMathLibrary.BreakRotator` (`SceneComponent.RelativeRotation` (`self.Cylinder`))))
  (`parent.ReceiveBeginPlay`)
  (set `self.TargetRotation` _relativerotation_yaw))

(event `Interact_1_1`
  (params (`Player Character` :type "/Game/BPs/BP_FirstPersonCharacter Object Reference") (PickUpActor :type "/Game/BPs/Pickups/BP_PickUpActor Object Reference")))

(event `self.ReceiveTick`
  (params (DeltaSeconds :type "Float (single-precision)"))
  (`SceneComponent.K2_SetRelativeRotation` (`self.Cylinder`) (`KismetMathLibrary.RLerp` (`SceneComponent.RelativeRotation` (`self.Cylinder`)) (`KismetMathLibrary.MakeRotator` 0.0 0.0 (`self.TargetRotation`)) (* (`GameplayStatics.GetWorldDeltaSeconds`) 15.0) true) false false))

(event `Interacted`
  (if (not (`self.NeedsItem`))
    (`self.Get RotationDirection`)
    (`self.SetTargetRotation`)
    (`GameplayStatics.PlaySound2D` (`self.SpinSound`) 1.0 1.0 0.0 null null)
    (`KismetSystemLibrary.Delay` 0.2)
    (bind _is_correct (`self.CheckIfCorrect`))
    (bind _output_get (set `self.Is Correct` _is_correct))
    (if _output_get
      (`GameplayStatics.PlaySound2D` (`self.CorrectRotSound`) 1.0 1.0 0.0 null null))
    (`self.GiveRotationBool` _output_get)))

(event `/Game/BPs/interfaces/BPI_ItemDialogueTextInterface.UpdateDisplayText`
  (params (PlayerCharacter :type "/Game/BPs/BP_FirstPersonCharacter Object Reference") (TypeOfText :type "/Game/BPs/interfaces/E_DialogueTypes Enum" :default "NewEnumerator0"))
  (bind _ingamehud (`/Game/BPs/BP_FirstPersonCharacter.IngameHUD` PlayerCharacter))
  (switch `/Game/BPs/interfaces/E_DialogueTypes` TypeOfText
    (:`NewEnumerator0`
      (set `self.Text` (`KismetArrayLibrary.Array_Random` (`self.MissingItemDialogue`))))
    (:`NewEnumerator1`
      (set `self.Text` (`KismetArrayLibrary.Array_Random` (`self.WrongItemDialogue`))))
    (:`NewEnumerator2`
      (set `self.Text` "")))
  (`/Game/BPs/Widgets/ComicsAndTuts/BP_Controlls.SetFulltext` _ingamehud (`self.Text`))
  (`/Game/BPs/Widgets/ComicsAndTuts/BP_Controlls.UpdateDialogueText` _ingamehud))

(event `Open`
  (bind _pivotlid (`self.PivotLid`))
  (bind (_relativerotation_roll _relativerotation_pitch _relativerotation_yaw) (`KismetMathLibrary.BreakRotator` (`SceneComponent.RelativeRotation` _pivotlid)))
  (bind (_direction _newtrack_0) (`Timeline|OpenLid` :!via `PlayFromStart`)
    (:`Update`
      (`SceneComponent.K2_SetRelativeRotation` _pivotlid (`KismetMathLibrary.MakeRotator` (`KismetMathLibrary.Lerp` 0.0 90.0 _newtrack_0) 0.0 _relativerotation_yaw) false false))))

(fn `CheckIfCorrect`
  (returns (`Is Correct` :type Boolean))
  (if (== (`self.TargetRotation`) (`self.CorrectRotation`))
    (`KismetSystemLibrary.PrintString` "YIPIEEEEEEE")
    (return true)
    (else
      (return false))))

(fn `Get RotationDirection`
  (bind (_location _rotation) (`Controller.GetPlayerViewPoint` (`GameplayStatics.GetPlayerController` 0)))
  (if (> (`KismetMathLibrary.Dot_VectorVector` (`KismetMathLibrary.Vector_Normal2D` (- (`self.K2_GetActorLocation`) _location)) (`KismetMathLibrary.Vector_Normal2D` (`KismetMathLibrary.GetRightVector` _rotation))) 0.0)
    (set `self.RotDirection` 1.0)
    (else
      (set `self.RotDirection` -1.0)))
  (return))

(fn `Interact`
  (params (`Player Character` :type "/Game/BPs/BP_FirstPersonCharacter Object Reference") (PickUpItem :type "/Game/BPs/BP_PickUpItem Object Reference"))
  (returns (UsedUpPickUp :type Boolean) (MultiUseItemused :type Boolean))
  (if (`self.CanBeInteractedW`)
    (`self.Interacted`)
    (`/Engine/EditorBlueprintResources/StandardMacros.IsValid` PickUpItem
      (:`Is Valid`
        (if (== PickUpItem (`self.CorrectItem`))
          (set `self.NeedsItem` false)
          (`/Game/BPs/BP_PickUpItem.ChangeParents` PickUpItem (`self.ItemPivot`))
          (return true false)
          (else
            (`self.UpdateDisplayText` `Player Character` "NewEnumerator1"))))
      (:`Is Not Valid`
        (if (`self.NeedsItem`)
          (`self.UpdateDisplayText` `Player Character` "NewEnumerator1"))))))

(fn `SetTargetRotation`
  (bind _returnvalue (+ (`self.TargetRotation`) (* 45.0 (`self.RotDirection`))))
  (`|ExecutionSequence`
    (:`then_0`
      (if (> _returnvalue 360.0)
        (set `self.TargetRotation` 0.0)))
    (:`then_1`
      (if (< _returnvalue 0.0)
        (set `self.TargetRotation` 360.0)))
    (:`then_2`
      (bind _output_get (set `self.TargetRotation` _returnvalue))
      (`KismetSystemLibrary.PrintString` (`KismetStringLibrary.Conv_DoubleToString` _output_get)))))

(fn `UserConstructionScript`
  (`parent.UserConstructionScript`))