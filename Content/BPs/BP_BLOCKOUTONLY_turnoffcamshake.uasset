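; Blockout-only interactable actor that toggles the first-person player character's camera shake.
; Its Interact function uses a FlipFlop to alternately set TurnOffCamShake true and false on the interacting character.
; It always reports that no pickup or multi-use item was used, and the event graph adds no logic of its own.
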(event `self.ReceiveBeginPlay`
  (`parent.ReceiveBeginPlay`))

(event `Interact_1_1`
  (params (`Player Character` :type "/Game/BPs/BP_FirstPersonCharacter Object Reference")))

(fn `Interact`
  (params (`Player Character` :type "/Game/BPs/BP_FirstPersonCharacter Object Reference") (PickUpItem :type "/Game/BPs/BP_PickUpItem Object Reference"))
  (returns (UsedUpPickUp :type Boolean) (MultiUseItemused :type Boolean))
  (set `self.As BP First Person Character` `Player Character`)
  (`/Engine/EditorBlueprintResources/StandardMacros.FlipFlop`
    (:`A`
      (set `/Game/BPs/BP_FirstPersonCharacter.TurnOffCamShake` true (`self.As BP First Person Character`)))
    (:`B`
      (set `/Game/BPs/BP_FirstPersonCharacter.TurnOffCamShake` false (`self.As BP First Person Character`))))
  (return false false))

(fn `UserConstructionScript`
  (`parent.UserConstructionScript`))