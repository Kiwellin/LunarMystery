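; Actor component that dissolves its owner's meshes with a matching Niagara particle effect.
; BeginPlay gathers spline meshes, or components of a configurable class without a spline, and creates two dynamic slot-0 materials each: mesh and particle.
; SpawnEmitter attaches a Niagara system to each mesh, passing its particle material.
; DissolveObject takes an external timeline value and sets DissolveAlpha on both sets, remapped for meshes; the built-in curve-driven dissolve is disconnected.
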(event `self.ReceiveTick`
  (params (DeltaSeconds :type "Float (single-precision)")))

(event `self.ReceiveBeginPlay`
  (bind _all_meshes (`self.CheckIfSplineOrStatic`))
  (bind _output_get (set `self.AllMeshes` _all_meshes))
  (for _array_element _output_get
    (bind _asmesh_component (cast `MeshComponent` _array_element))
    (bind _output_get_2 (set `self.CurrentMesh` _asmesh_component))
    (`KismetArrayLibrary.Array_Add` (`self.currentmesharray`) _output_get_2)
    (bind _output_get_3 (set `self.Material` (`PrimitiveComponent.GetMaterial` _asmesh_component 0)))
    (`KismetArrayLibrary.Array_Add` (`self.materialarray`) _output_get_3))
  (`|ExecutionSequence`
    (:`then_0`
      (for (_array_element_2 _array_index) (`self.materialarray`)
        (bind _returnvalue (`KismetMaterialLibrary.CreateDynamicMaterialInstance` _array_element_2))
        (bind _output_get_4 (set `self.ComponentMaterial` _returnvalue))
        (`KismetArrayLibrary.Array_Add` (`self.ComponentMaterialarray`) _output_get_4)
        (`MaterialInstanceDynamic.SetScalarParameterValue` _output_get_4 "DissolveAlpha" 0.0)
        (`PrimitiveComponent.SetMaterial` (`|GetArrayItem` (`self.currentmesharray`) _array_index) 0 _output_get_4)))
    (:`then_1`
      (for _array_element_3 (`self.materialarray`)
        (bind _returnvalue_2 (`KismetMaterialLibrary.CreateDynamicMaterialInstance` _array_element_3))
        (bind _output_get_5 (set `self.ParticleMaterial` _returnvalue_2))
        (`KismetArrayLibrary.Array_Add` (`self.Particlearray`) _output_get_5)
        (`MaterialInstanceDynamic.SetScalarParameterValue` _output_get_5 "IsParticle" 1.0)
        (`MaterialInstanceDynamic.SetScalarParameterValue` _output_get_5 "DissolveAlpha" 0.0)))))

(event `SpawnEmitter`
  (for (_array_element _array_index) (`self.currentmesharray`)
    (bind _returnvalue (`NiagaraFunctionLibrary.SpawnSystemAttached` (`self.System Template`) _array_element "None" (0.0 0.0 0.0) (struct) "KeepRelativeOffset"))
    (`NiagaraComponent.SetVariableMaterial` _returnvalue "Material" (`|GetArrayItem` (`self.Particlearray`) _array_index))))

(fn `CheckIfSplineOrStatic`
  (returns (`All meshes` :type "Array of SceneComponent Object Reference"))
  (locals (ArrayOfStaticMesh :type "Array of MeshComponent Object Reference"))
  (bind _returnvalue (`self.GetOwner`))
  (bind _returnvalue_2 (`Actor.GetComponentByClass` _returnvalue "/Script/Engine.SplineComponent"))
  (`/Engine/EditorBlueprintResources/StandardMacros.IsValid` _returnvalue_2
    (:`Is Valid`
      (set `self.spline` _returnvalue_2)
      (return (`Actor.K2_GetComponentsByClass` _returnvalue "/Script/Engine.SplineMeshComponent")))
    (:`Is Not Valid`
      (return (`Actor.K2_GetComponentsByClass` _returnvalue (`self.Component Class`))))))

(fn `DissolveObject`
  (params (Timeline :type "Float (double-precision)"))
  (`|ExecutionSequence`
    (:`then_0`
      (for _array_element (`self.Particlearray`)
        (`MaterialInstanceDynamic.SetScalarParameterValue` _array_element "DissolveAlpha" Timeline)))
    (:`then_1`
      (for _array_element_2 (`self.ComponentMaterialarray`)
        (`MaterialInstanceDynamic.SetScalarParameterValue` _array_element_2 "DissolveAlpha" (`KismetMathLibrary.MapRangeClamped` Timeline 0.0 1.0 -0.5 1.0))))))