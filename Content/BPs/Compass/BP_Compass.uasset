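; BP_Compass is a compass actor that turns its Scene component to indicate north relative to the player's view.
; BeginPlay caches the location of the Northmarker reference as NorthLocation; a GetActorOfClass lookup for BP_Northmarker exists but is not wired to run.
; Each Tick, it sets Scene's relative yaw to the negated difference between the player's control yaw and the look-at yaw from the compass to north.
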(event `self.ReceiveBeginPlay`
  (`parent.ReceiveBeginPlay`)
  (set `self.NorthLocation` (`self.K2_GetActorLocation` (`self.Northmarker`))))

(event `self.ReceiveTick`
  (params (DeltaSeconds :type "Float (single-precision)"))
  (bind (_returnvalue_roll _returnvalue_pitch _returnvalue_yaw) (`KismetMathLibrary.BreakRotator` (`Pawn.GetControlRotation` (`GameplayStatics.GetPlayerPawn` 0))))
  (bind (_returnvalue_roll_2 _returnvalue_pitch_2 _returnvalue_yaw_2) (`KismetMathLibrary.BreakRotator` (`KismetMathLibrary.FindLookAtRotation` (`self.K2_GetActorLocation`) (`self.NorthLocation`))))
  (`SceneComponent.K2_SetRelativeRotation` (`self.Scene`) (`KismetMathLibrary.MakeRotator` 0.0 0.0 (* (- _returnvalue_yaw _returnvalue_yaw_2) -1.0)) false false))

(fn `UserConstructionScript`
  (`parent.UserConstructionScript`))