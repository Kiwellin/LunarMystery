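; Sorting puzzle chest whose lid opens in stages as items are correctly placed on four linked place-item targets.
; On BeginPlay it binds to each target's events, raising the correct count on a correct placement and lowering it on pickup.
; The count sets the lid angle exponentially, as LidOpenFull raised to the fraction of four, negated.
; A timeline rotates the Pivot's roll from the previous angle to the new one.
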(event `self.ReceiveBeginPlay`
  (bind _placeitemtarget_01 (`self.PlaceItemTarget_01`))
  (add `/Game/BPs/InventoryAndPlacePuzzle/BP_PlaceItemTarget.CheckIfAllCorrect` _placeitemtarget_01 (delegate `OpenMore`))
  (add `/Game/BPs/InventoryAndPlacePuzzle/BP_PlaceItemTarget.CheckIfAllCorrect` (`self.PlaceItemTarget_02`) (delegate `OpenMore`))
  (add `/Game/BPs/InventoryAndPlacePuzzle/BP_PlaceItemTarget.CheckIfAllCorrect` (`self.PlaceItemTarget_04`) (delegate `OpenMore`))
  (add `/Game/BPs/InventoryAndPlacePuzzle/BP_PlaceItemTarget.CheckIfAllCorrect` (`self.PlaceItemTarget_03`) (delegate `OpenMore`))
  (add `/Game/BPs/InventoryAndPlacePuzzle/BP_SortingPuzzlePlace.PickedUpItem` _placeitemtarget_01 (delegate `CloseABit`))
  (add `/Game/BPs/InventoryAndPlacePuzzle/BP_SortingPuzzlePlace.PickedUpItem` (`self.PlaceItemTarget_02`) (delegate `CloseABit`))
  (add `/Game/BPs/InventoryAndPlacePuzzle/BP_SortingPuzzlePlace.PickedUpItem` (`self.PlaceItemTarget_03`) (delegate `CloseABit`))
  (add `/Game/BPs/InventoryAndPlacePuzzle/BP_SortingPuzzlePlace.PickedUpItem` (`self.PlaceItemTarget_04`) (delegate `CloseABit`)))

(event `OpenMore`
  (`self.ChangeCorrectStones` 1)
  (`self.Play`))

(event `CloseABit`
  (`self.ChangeCorrectStones` -1)
  (`self.Play`))

(event `Play`
  (set `self.AddMoreOpen` (/ (`KismetMathLibrary.Conv_IntToDouble` (`self.CorrectStones`)) 4.0))
  (set `self.OpenAmount` (* (`KismetMathLibrary.MultiplyMultiply_FloatFloat` (`self.LidOpenFull`) (`self.AddMoreOpen`)) -1.0))
  (bind (_direction _newtrack_0) (`Timeline|OpenChestMore` :!via `PlayFromStart`)
    (:`Update`
      (`SceneComponent.K2_SetRelativeRotation` (`self.pivot`) (`KismetMathLibrary.MakeRotator` (`KismetMathLibrary.Lerp` (`self.OldAmount`) (`self.OpenAmount`) _newtrack_0)) false false))
    (:`Finished`
      (set `self.OldAmount` (`self.OpenAmount`)))))

(fn `ChangeCorrectStones`
  (params (Add :type Integer))
  (bind _output_get (set `self.CorrectStones` (+ (`self.CorrectStones`) Add)))
  (`KismetSystemLibrary.PrintString` (`KismetStringLibrary.Conv_IntToString` _output_get)))

(fn `UserConstructionScript`)