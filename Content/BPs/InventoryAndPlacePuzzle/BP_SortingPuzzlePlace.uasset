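; Sorting puzzle placement spot, a child Blueprint that inherits its item-placing interaction from its parent.
; Interact forwards to the parent and returns its UsedUpPickUp result, while always reporting that no multi-use item was used.
; RemoveStone fires the PickedUpItem dispatcher, then clears the ItemCorrect flag.
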(event `RemoveStone`
  (`self.PickedUpItem`)
  (set `self.ItemCorrect` false))

(fn `Interact`
  (params (`Player Character` :type "/Game/BPs/BP_FirstPersonCharacter Object Reference") (PickUpItem :type "/Game/BPs/BP_PickUpItem Object Reference"))
  (returns (UsedUpPickUp :type Boolean) (MultiUseItemused :type Boolean))
  (bind _useduppickup (`parent.Interact` `Player Character` PickUpItem))
  (return _useduppickup false))

(fn `UserConstructionScript`
  (`parent.UserConstructionScript`))