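; Interactable placement target for the item puzzle that holds one pickup on its PlaceBowlHere component and checks whether it is correct.
; Interact attaches the item to an empty slot and compares it to CorrectItem; hint-pin targets instead filter for HintNote items and count them correct immediately.
; A correct placement fires the puzzle dispatchers, then either disables the item's collision or, for re-pickable pinned notes, shifts the mesh.
; The offering-bowl ingredient check is unwired.
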(event `self.ReceiveBeginPlay`)

(event `CheckPlacedItem`
  (if (== (`self.PlacedItem`) (`self.CorrectItem`))
    (`self.ItemIsCorrect`)
    (set `self.ItemCorrect` true)))

(event `ItemIsCorrect`
  (`self.CheckIfAllCorrect`)
  (`self.ItemPlacedCorrect`)
  (if (`self.CanPickUpItemAgain`)
    (if (`self.TargetIsNote/HintPin?`)
      (bind _asbp_hint_note (cast `/Game/BPs/HintsAndNotes/BP_HintNote` (`self.PlacedItem`)))
      (bind _relativelocation_x (`KismetMathLibrary.BreakVector` (`SceneComponent.RelativeLocation` (`/Game/BPs/HintsAndNotes/BP_HintNote.PinLoc` _asbp_hint_note))))
      (`KismetSystemLibrary.PrintString` (`KismetStringLibrary.Conv_DoubleToString` _relativelocation_x))
      (`SceneComponent.K2_SetRelativeLocation` (`/Game/BPs/BP_PickUpItem.StaticMesh` _asbp_hint_note) (`KismetMathLibrary.MakeVector` (`KismetMathLibrary.Abs` _relativelocation_x)) false false))
    (else
      (`self.SetActorEnableCollision` (`self.PlacedItem`) false))))

(fn `CheckIfItemIsHint/NoteClass`
  (params (PickUpItem :type "/Game/BPs/BP_PickUpItem Object Reference"))
  (returns (ReturnValue :type Boolean))
  (bind _returnvalue (`KismetMathLibrary.ClassIsChildOf` (`GameplayStatics.GetObjectClass` PickUpItem) (`self.HintNote`)))
  (if (`self.NeedsRunicCode?`)
    (if (== PickUpItem (`self.CorrectItem`))
      (return _returnvalue))
    (elif _returnvalue
      (return _returnvalue))))

(fn `CheckIfItemIsOfferingBowl`
  (returns (ReturnValue :type Boolean))
  (bind _asbp_offering_bowl (cast `/Game/BPs/Sacrifice/BP_OfferingBowl` (`self.PlacedItem`))
    (:`then`
      (bind _addedingredient (`/Game/BPs/Sacrifice/BP_OfferingBowl.AddedIngredient` _asbp_offering_bowl))
      (`/Engine/EditorBlueprintResources/StandardMacros.IsValid` _addedingredient
        (:`Is Valid`
          (if (== (`GameplayStatics.GetObjectClass` _addedingredient) (`self.CorrectIngredient`))
            (return true)))
        (:`Is Not Valid`
          (return false))))
    (:`CastFailed`
      (return true))))

(fn `Interact`
  (params (`Player Character` :type "/Game/BPs/BP_FirstPersonCharacter Object Reference") (PickUpItem :type "/Game/BPs/BP_PickUpItem Object Reference"))
  (returns (UsedUpPickUp :type Boolean) (MultiUseItemused :type Boolean))
  (`/Engine/EditorBlueprintResources/StandardMacros.IsValid` (`SceneComponent.GetChildComponent` (`self.PlaceBowlHere`) 0)
    (:`Is Not Valid`
      (`/Engine/EditorBlueprintResources/StandardMacros.IsValid` PickUpItem
        (:`Is Valid`
          (if (`self.TargetIsNote/HintPin?`)
            (bind _returnvalue (`self.CheckIfItemIsHint/NoteClass` PickUpItem))
            (if _returnvalue
              (`self.PlaceItem` PickUpItem)
              (`self.ItemIsCorrect`)
              (return true false))
            (else
              (`self.PlaceItem` PickUpItem)
              (`self.CheckPlacedItem`)
              (return true false))))))))

(fn `PlaceItem`
  (params (PlacedItem :type "/Game/BPs/BP_PickUpItem Object Reference"))
  (bind _output_get (set `self.PlacedItem` PlacedItem))
  (`/Game/BPs/BP_PickUpItem.ChangeParents` _output_get (`self.PlaceBowlHere`))
  (`PrimitiveComponent.SetCollisionEnabled` (`/Game/BPs/BP_PickUpItem.StaticMesh` PlacedItem) "QueryAndPhysics"))

(fn `UserConstructionScript`)