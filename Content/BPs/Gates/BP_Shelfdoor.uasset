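; Shelf door actor that swings open when its linked lock is solved or opened.
; On BeginPlay it binds its open event to a SpinLock's solved event if one is set, otherwise to a NormalLock's opened event.
; The open event plays a timeline that lerps the pivot's yaw from zero to a configurable open amount.
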(event `self.ReceiveBeginPlay`
  (bind _spinlock (`self.SpinLock`))
  (`/Engine/EditorBlueprintResources/StandardMacros.IsValid` _spinlock
    (:`Is Valid`
      (add `/Game/BPs/Spinlock/BP_SpinLockPawn.SolvedPuzzle` _spinlock (delegate `OpenGate_Event`)))
    (:`Is Not Valid`
      (add `/Game/BPs/NormalLocksNKeys/BP_ShelfLockNormal.Opened` (`self.NormalLock`) (delegate `OpenGate_Event`)))))

(event `OpenGate_Event`
  (bind (_direction _newtrack_0) (`Timeline|Timeline`)
    (:`Update`
      (`SceneComponent.K2_SetRelativeRotation` (`self.Pivot`) (`KismetMathLibrary.MakeRotator` 0.0 0.0 (`KismetMathLibrary.Lerp` 0.0 (`self.OpenAmount`) _newtrack_0)) false false))))

(fn `UserConstructionScript`)