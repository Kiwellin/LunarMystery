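; BP_MainGateCheck is a level actor that opens the main gate once three vines have dissolved.
; On BeginPlay it binds a single handler to the Dissolved dispatcher of Vine1, Vine2 and Vine3.
; Each call increments a SolvedPlates counter, and when it reaches three the actor calls the Opengates dispatcher for listeners to respond.
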(event `self.ReceiveBeginPlay`
  (add `/Game/BPs/Gates/Vines/BP_VineMeshOverSpline.Dissolved` (`self.Vine1`) (delegate `Dissolved_Event`))
  (add `/Game/BPs/Gates/Vines/BP_VineMeshOverSpline.Dissolved` (`self.Vine3`) (delegate `Dissolved_Event`))
  (add `/Game/BPs/Gates/Vines/BP_VineMeshOverSpline.Dissolved` (`self.Vine2`) (delegate `Dissolved_Event`)))

(event `Dissolved_Event`
  (bind _output_get (set `self.SolvedPlates` (+ (`self.SolvedPlates`) 1)))
  (if (== _output_get 3)
    (`self.Opengates`)))

(fn `UserConstructionScript`)