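; Vine gate actor that dissolves and removes itself when its linked rune plate reports a correct code.
; On that callback, BPTransitionComponent1 spawns an emitter and a Dissolve timeline drives its dissolve effect.
; When the timeline finishes, the actor calls Dissolved, then destroys itself after a short delay.
; The construction script's logic for tiling spline meshes along a spline is disconnected, so it never runs.
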(event `self.ReceiveBeginPlay`
  (add `/Game/BPs/RunePlateTest/BP_RunePlatePawn.CodeCorrect` (`self.RunePlate Solved`) (delegate `CodeCorrect_Event`)))

(event `CodeCorrect_Event`
  (`/Game/BPs/Niagara/BP_TransitionComponent.SpawnEmitter` (`self.BP_TransitionComponent1`))
  (bind (_direction _dissolvealpha) (`Timeline|dissolve`)
    (:`Update`
      (`/Game/BPs/Niagara/BP_TransitionComponent.DissolveObject` (`self.BP_TransitionComponent1`) _dissolvealpha))
    (:`Finished`
      (`self.Dissolved`)
      (`KismetSystemLibrary.Delay` 0.2)
      (`self.K2_DestroyActor`))))

(fn `UserConstructionScript`)