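; BP_InteractTextComponent is an actor component that supplies interaction text to the player's inspection mode widget.
; On BeginPlay it gathers every component of its own class on the owner, so an actor can carry several lines.
; SetFullText sends the InteractText at the current index to the widget, then calls IndexDialogue to advance the index, resetting at the array's end.
; UpdateDisplayText tells the widget to update its dialogue text.
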(event `self.ReceiveBeginPlay`
  (set `self.Interactiontexts` (`Actor.K2_GetComponentsByClass` (`self.GetOwner`) "BP_InteractTextComponent_C")))

(event `/Game/BPs/interfaces/BPI_ItemDialogueTextInterface.SetFullText`
  (params (PlayerCharacter :type "/Game/BPs/BP_FirstPersonCharacter Object Reference"))
  (`/Game/BPs/Widgets/WB_3DOverlay.SetFulltext` (`/Game/BPs/BP_FirstPersonCharacter.InspectionModeWidget` PlayerCharacter) (`/Game/BPs/Components/BP_InteractTextComponent.InteractText` (`|GetArrayItem` (`self.Interactiontexts`) (`self.DialogueIndex`))))
  (`self.IndexDialogue` 1))

(event `/Game/BPs/interfaces/BPI_ItemDialogueTextInterface.UpdateDisplayText`
  (params (PlayerCharacter :type "/Game/BPs/BP_FirstPersonCharacter Object Reference") (TypeOfText :type "/Game/BPs/interfaces/E_DialogueTypes Enum" :default "NewEnumerator0"))
  (`/Game/BPs/Widgets/WB_3DOverlay.UpdateDialogueText` (`/Game/BPs/BP_FirstPersonCharacter.InspectionModeWidget` PlayerCharacter)))

(fn `IndexDialogue`
  (params (DialogueIndex :type Integer))
  (set `self.DialogueIndex` (+ DialogueIndex (`self.DialogueIndex`)))
  (if (== (`self.DialogueIndex`) (`KismetArrayLibrary.Array_Length` (`self.Interactiontexts`)))
    (set `self.DialogueIndex` 0)))