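; Possessable bell puzzle where the player selects and rings four bells to reproduce sound codes, unlocked by a specific pickup that reveals the missing bell.
; Navigation input cycles a highlighted selection, and interacting plays that bell's sound and appends its value to the entered code.
; Each entry is checked as a prefix of the current DataTable row, resetting and re-showing the code on mistakes.
; Completing the final row solves the puzzle and releases the player.
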(event `self.ReceiveBeginPlay`
  (`parent.ReceiveBeginPlay`)
  (set `self.Bells` (`|MakeArray` (`self.Bell1`) (`self.Bell2`) (`self.Bell3`) (`self.Bell4`)))
  (bind _outrownames (`DataTableFunctionLibrary.GetDataTableRowNames` (`self.DT Sound Codes`)))
  (bind _output_get (set `self.Out Row Names` _outrownames))
  (bind _returnvalue (`|GetDataTableRow` (`self.DT Sound Codes`) (`|GetArrayItem` _output_get (`self.CodeIndex`)))
    (:`then`
      (set `self.OutRow` _returnvalue)
      (`self.SetNextCode`))))

(event `EnhancedInput|/Game/Input/Actions/IA_ExitPuzzle`
  (params (ActionValue :type Boolean) (ElapsedSeconds :type "Float (double-precision)") (TriggeredSeconds :type "Float (double-precision)") (InputAction :type "InputAction Object Reference" :default "/Game/Input/Actions/IA_ExitPuzzle.IA_ExitPuzzle"))
  (:`Triggered`
    (`self.Return to Character`)))

(event `EnhancedInput|/Game/Input/Actions/IA_NavigateRight`
  (params (ActionValue :type Boolean) (ElapsedSeconds :type "Float (double-precision)") (TriggeredSeconds :type "Float (double-precision)") (InputAction :type "InputAction Object Reference" :default "/Game/Input/Actions/IA_NavigateRight.IA_NavigateRight"))
  (:`Triggered`
    (if (`self.CanSelectNext`)
      (`self.Navigate Bells` 1))))

(event `self.Return to Character`
  (`parent.Return to Character`)
  (`self.UpdateHighlightOfSelectedBell` false))

(event `EnhancedInput|/Game/Input/Actions/IA_NavigateLeft`
  (params (ActionValue :type Boolean) (ElapsedSeconds :type "Float (double-precision)") (TriggeredSeconds :type "Float (double-precision)") (InputAction :type "InputAction Object Reference" :default "/Game/Input/Actions/IA_NavigateLeft.IA_NavigateLeft"))
  (:`Triggered`
    (if (`self.CanSelectNext`)
      (`self.Navigate Bells` -1))))

(event `EnhancedInput|/Game/Input/Actions/IA_Interact`
  (params (ActionValue :type Boolean) (ElapsedSeconds :type "Float (double-precision)") (TriggeredSeconds :type "Float (double-precision)") (InputAction :type "InputAction Object Reference" :default "/Game/Input/Actions/IA_Interact.IA_Interact"))
  (:`Triggered`
    (if (`self.CanSelectNext`)
      (`TimelineComponent.SetPlayRate` (`self.Movebell`) 5.0)
      (`TimelineComponent.PlayFromStart` (`self.Movebell`))
      (`GameplayStatics.PlaySoundAtLocation` (`BlueprintMapLibrary.Map_Find` (`self.BellSoundTable`) (`self.CurrentPieceIndex`)) (`self.K2_GetActorLocation`) (struct) 1.0 1.0 0.0 null null null null)
      (bind _addednumber (`self.AddToCode`))
      (if _addednumber
        (bind _is_correct (`self.CheckCode`))
        (if _is_correct
          (`KismetSystemLibrary.PrintString` "going to next code")
          (set `self.CanSelectNext` false)
          (`self.ClearCode`)
          (bind _lastcode (`self.GoToNextCode`))
          (if _lastcode
            (`self.UpdateHighlightOfSelectedBell` false)
            (set `self.CanBePossessed` false)
            (`self.Return to Character`)
            (`self.PuzzleSolved`)
            (else
              (`self.SetNextCode`)
              (`self.ShowCode`)
              (set `self.CanSelectNext` true))))))))

(fn `AddToCode`
  (returns (AddedNumber :type Boolean))
  ; Get Code  length
  (bind _outcolumnnames (`DataTableFunctionLibrary.GetDataTableColumnNames` (`self.DT Sound Codes`)))
  (set `self.Out Column Names` _outcolumnnames)
  (`KismetArrayLibrary.Array_Add` (`self.CurrentCode`) (`/Game/BPs/BellPuzzle/BP_SMBell.SoundInt` (`self.GetSelectedBell`)))
  (set `self.CodeLengthIndex` (+ (`self.CodeLengthIndex`) 1))
  (return true))

(fn `CheckCode`
  (returns (`is correct` :type Boolean))
  (locals (NewLocalVar :type "Array of Integer"))
  (bind _output_get (set `self.PartialCode` (`self.Code`)))
  (`KismetArrayLibrary.Array_Resize` _output_get (`self.CodeLengthIndex`))
  (if (`KismetArrayLibrary.Array_Identical` (`self.PartialCode`) (`self.CurrentCode`))
    (if (== (`KismetArrayLibrary.Array_Length` (`self.CurrentCode`)) (`KismetArrayLibrary.Array_Length` (`self.Out Column Names`)))
      (`KismetSystemLibrary.PrintString` "is correct")
      (return true)
      (else
        _))
    (else
      (`KismetSystemLibrary.PrintString` "INCORRECT")
      (`self.ClearCode`)
      (`self.ShowCode`)))
  (return false))

(fn `CheckForBell`
  (params (PickUpItem :type "/Game/BPs/BP_PickUpItem Object Reference"))
  (returns (UsedPickup :type Boolean))
  (`/Engine/EditorBlueprintResources/StandardMacros.IsValid` PickUpItem
    (:`Is Valid`
      (if (== PickUpItem (`self.CorrectItem`))
        (set `self.CanBePossessed` true)
        (`/Game/BPs/BP_PickUpItem.DestroySelf` PickUpItem)
        (`self.UnhideLastBell`)
        (set `self.NeedsItem` false)
        (return true)
        (else
          (return false))))))

(fn `ClearCode`
  (set `self.CodeLengthIndex` 0)
  (`KismetArrayLibrary.Array_Clear` (`self.PartialCode`))
  (`KismetArrayLibrary.Array_Clear` (`self.CurrentCode`)))

(fn `GetSelectedBell`
  (returns (Output :type "/Game/BPs/BellPuzzle/BP_SMBell Object Reference"))
  (return (`|GetArrayItem` (`self.Bells`) (`self.CurrentPieceIndex`))))

(fn `GoToNextCode`
  (returns (LastCode :type Boolean))
  (bind _codeindex (`self.CodeIndex`))
  (if (< _codeindex (`KismetArrayLibrary.Array_LastIndex` (`self.Out Row Names`)))
    (bind _output_get (set `self.CodeIndex` (+ _codeindex 1)))
    (bind _returnvalue (`|GetDataTableRow` (`self.DT Sound Codes`) (`|GetArrayItem` (`self.Out Row Names`) _output_get))
      (:`then`
        (set `self.OutRow` _returnvalue)
        (return false)))
    (else
      (return true))))

(fn `Interact`
  (params (`Player Character` :type "/Game/BPs/BP_FirstPersonCharacter Object Reference") (PickUpItem :type "/Game/BPs/BP_PickUpItem Object Reference"))
  (returns (UsedUpPickUp :type Boolean) (MultiUseItemused :type Boolean))
  (if (`self.CanBePossessed`)
    (`parent.Interact` `Player Character` PickUpItem)
    (`self.UpdateHighlightOfSelectedBell` true)
    (`self.ShowCode`)
    (return false false)
    (else
      (bind _usedpickup (`self.CheckForBell` PickUpItem))
      (return _usedpickup false))))

(fn `Navigate Bells`
  (params (Direction :type Integer))
  (`self.UpdateHighlightOfSelectedBell` false)
  (set `self.CurrentPieceIndex` (+ (`self.CurrentPieceIndex`) Direction))
  (`|ExecutionSequence`
    (:`then_0`
      ;[1 1 1] Make sure index not too high
      (if (> (`self.CurrentPieceIndex`) (`KismetArrayLibrary.Array_LastIndex` (`self.Bells`)))
        (set `self.CurrentPieceIndex` (- (`self.CurrentPieceIndex`) (`KismetArrayLibrary.Array_Length` (`self.Bells`))))))
    (:`then_1`
      ;[1 1 1] Make sure index not too low
      (if (< (`self.CurrentPieceIndex`) 0)
        (set `self.CurrentPieceIndex` (+ (`self.CurrentPieceIndex`) (`KismetArrayLibrary.Array_Length` (`self.Bells`))))))
    (:`then_2`
      ;[1 1 1] Update highlight
      (`self.UpdateHighlightOfSelectedBell` true))))

(fn `SetNextCode`
  (bind (_outrow_sound1 _outrow_sound2 _outrow_sound3 _outrow_sound4) (break `/Game/BPs/BellPuzzle/S_SoundCode` (`self.OutRow`)))
  (`KismetArrayLibrary.Array_Clear` (`self.Code`))
  (set `self.Code` (`|MakeArray` _outrow_sound1 _outrow_sound2 _outrow_sound3 _outrow_sound4)))

(fn `UnhideLastBell`
  (`SceneComponent.SetVisibility` (`self.Bell3`) true false))

(fn `UpdateHighlightOfSelectedBell`
  (params (bEnabled :type Boolean))
  (`MeshComponent.SetOverlayMaterial` (`self.GetSelectedBell`) (select `bool` bEnabled :`true` "/Game/Materials/MI_ButtonHighlight.MI_ButtonHighlight" :!type "MaterialInterface Object Reference")))

(fn `UserConstructionScript`
  (`parent.UserConstructionScript`))