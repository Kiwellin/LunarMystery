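; A cat statue in the bell puzzle that voices the puzzle code as sounds, then dissolves and opens a chest when the puzzle is solved.
; A looping timer starts paused; the BellPuzzle show-code event unpauses it to play one looked-up sound per code entry, pausing again after the last.
; The solved event drives a transition component's emitter and timeline dissolve before opening the chest and destroying the statue.
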(event `self.ReceiveBeginPlay`
  (add `/Game/BPs/BellPuzzle/BP_BellPuzzle.PuzzleSolved` (`self.BellPuzzle`) (delegate `Destroy`))
  (add `/Game/BPs/BellPuzzle/BP_BellPuzzle.ShowCode` (`self.BellPuzzle`) (delegate `ShowNumbers`))
  (bind _returnvalue (`KismetSystemLibrary.K2_SetTimerDelegate` (delegate `Test`) 1.0 true))
  (bind _output_get (set `self.NewVar` _returnvalue))
  (`KismetSystemLibrary.K2_PauseTimerHandle` _output_get :!label _label))

(event `Test`
  (bind _code (`/Game/BPs/BellPuzzle/BP_BellPuzzle.Code` (`self.BellPuzzle`)))
  (if (== (`self.CodeIndexLocal`) (`KismetArrayLibrary.Array_Length` _code))
    (set `self.CodeIndexLocal` 0)
    (goto _label)
    (else
      (`KismetSystemLibrary.Delay` 0.3)
      (`GameplayStatics.PlaySoundAtLocation` (`BlueprintMapLibrary.Map_Find` (`self.CatSoundTable`) (`|GetArrayItem` _code (`self.CodeIndexLocal`))) (`self.K2_GetActorLocation`) (struct) 1.0 1.0 0.0 null null null null)
      (`KismetSystemLibrary.Delay` 0.3)
      (set `self.CodeIndexLocal` (+ (`self.CodeIndexLocal`) 1)))))

(event `ShowNumbers`
  (`KismetSystemLibrary.K2_UnPauseTimerHandle` (`self.NewVar`)))

(event `Destroy`
  (`/Game/BPs/Niagara/BP_TransitionComponent.SpawnEmitter` (`self.BP_TransitionComponent`))
  (bind (_direction _newtrack_0) (`Timeline|Timeline`)
    (:`Update`
      (`/Game/BPs/Niagara/BP_TransitionComponent.DissolveObject` (`self.BP_TransitionComponent`) _newtrack_0))
    (:`Finished`
      (`KismetSystemLibrary.Delay` 0.2)
      (`/Game/BPs/Spinlock/ChestWSpinlock/BP_BigChestMesh.OpenChest` (`self.Chest`))
      (`self.K2_DestroyActor`))))

(fn `UserConstructionScript`)