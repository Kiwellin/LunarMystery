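; BP_RunePlateSockel is an interactable socket that accepts the correct pickup item and reveals a rune plate in its place.
; On Interact, a matching item is reparented to the placement point, then immediately destroyed, and the referenced RunePlate is unhidden with collision enabled.
; A missing or wrong item shows a random dialogue line on the player's HUD.
; Pawn spawning, keypad collision and timed text clearing are left disconnected.
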(event `SpawnThePawn`
  (bind _runeplate (`self.RunePlate`))
  (bind _item (`self.Item`))
  (`self.K2_DetachFromActor` _item "KeepRelative" "KeepRelative" "KeepRelative")
  (`self.K2_DestroyActor` _item)
  (`self.SetActorHiddenInGame` _runeplate false)
  (`self.SetActorEnableCollision` _runeplate true))

(event `/Game/BPs/interfaces/BPI_ItemDialogueTextInterface.UpdateDisplayText`
  (params (PlayerCharacter :type "/Game/BPs/BP_FirstPersonCharacter Object Reference") (TypeOfText :type "/Game/BPs/interfaces/E_DialogueTypes Enum" :default "NewEnumerator0"))
  (bind _ingamehud (`/Game/BPs/BP_FirstPersonCharacter.IngameHUD` PlayerCharacter))
  (switch `/Game/BPs/interfaces/E_DialogueTypes` TypeOfText
    (:`NewEnumerator0`
      (set `self.Text` (`KismetArrayLibrary.Array_Random` (`self.MissingItemDialogue`))))
    (:`NewEnumerator1`
      (set `self.Text` (`KismetArrayLibrary.Array_Random` (`self.WrongItemDialogue`))))
    (:`NewEnumerator2`
      (set `self.Text` "")))
  (`/Game/BPs/Widgets/ComicsAndTuts/BP_Controlls.SetFulltext` _ingamehud (`self.Text`))
  (`/Game/BPs/Widgets/ComicsAndTuts/BP_Controlls.UpdateDialogueText` _ingamehud))

(fn `Interact`
  (params (`Player Character` :type "/Game/BPs/BP_FirstPersonCharacter Object Reference") (PickUpItem :type "/Game/BPs/BP_PickUpItem Object Reference"))
  (returns (UsedUpPickUp :type Boolean) (MultiUseItemused :type Boolean))
  (`/Engine/EditorBlueprintResources/StandardMacros.IsValid` PickUpItem
    (:`Is Valid`
      (if (== PickUpItem (`self.CorrectItem`))
        (bind _output_get (set `self.Item` PickUpItem))
        (`/Game/BPs/BP_PickUpItem.ChangeParents` _output_get (`self.PlaceRunePlateHERE`))
        (`self.SpawnThePawn`)
        (return true false)
        (else
          (`self.UpdateDisplayText` `Player Character` "NewEnumerator1"))))
    (:`Is Not Valid`
      (`self.UpdateDisplayText` `Player Character`))))

(fn `UserConstructionScript`)