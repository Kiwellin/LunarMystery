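; Decal actor in the LevelSequences folder that animates a text reveal through a material parameter.
; On BeginPlay it creates a dynamic instance of the decal's material, prints its name and assigns it back to the decal.
; The Play event runs a timeline from the start, driving the "Appear" scalar on that instance each update.
; Several unconnected text and mesh material nodes are left unused.
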(event `self.ReceiveBeginPlay`
  (bind _decal (`self.Decal`))
  (bind _returnvalue (`KismetMaterialLibrary.CreateDynamicMaterialInstance` (`DecalComponent.GetDecalMaterial` _decal)))
  (bind _output_get (set `self.mid` _returnvalue))
  (`KismetSystemLibrary.PrintString` (`KismetSystemLibrary.GetDisplayName` _output_get))
  (`DecalComponent.SetDecalMaterial` _decal _output_get))

(event `Play`
  (bind (_direction _newtrack_0) (`Timeline|Timeline` :!via `PlayFromStart`)
    (:`Update`
      (`MaterialInstanceDynamic.SetScalarParameterValue` (`self.mid`) "Appear" _newtrack_0))))

(fn `UserConstructionScript`)