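; BP_RandomAtmoSound is an atmosphere sound actor that plays its Audio component at random intervals.
; BeginPlay schedules the first Play event after a random delay, with a wider range than later intervals.
; Each Play starts the sound, prints a new random delay and sets the timer again with looping enabled.
; An unused SetTimer event and a disconnected timer-clearing call remain in the graph.
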(event `self.ReceiveBeginPlay`
  (set `self.Time` (`KismetMathLibrary.RandomFloatInRange` 10.0 300.0))
  (bind _returnvalue (`KismetSystemLibrary.K2_SetTimerDelegate` (delegate `Play`) (`self.Time`))))

(event `Play`
  (`AudioComponent.Play` (`self.Audio`) 0.0)
  (bind _output_get (set `self.Time` (`KismetMathLibrary.RandomFloatInRange` 10.0 100.0)))
  (`KismetSystemLibrary.PrintString` (`KismetStringLibrary.Conv_DoubleToString` _output_get))
  (`KismetSystemLibrary.K2_SetTimerDelegate` (delegate `Play`) (`self.Time`) true))

(event `SetTimer`
  (bind _output_get (set `self.Time` (`KismetMathLibrary.RandomFloatInRange` 5.0 15.0)))
  (`KismetSystemLibrary.PrintString` (`KismetStringLibrary.Conv_DoubleToString` _output_get)))

(fn `UserConstructionScript`)